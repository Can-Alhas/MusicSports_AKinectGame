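; BP_Cam is a camera actor that becomes the first player controller's view target when play begins.
; BeginPlay also caches the player character reference.
; A helper function computes an interpolated look-at rotation from the camera toward the player, but the node applying it is disconnected and Tick is empty, so the Blueprint never rotates the camera.
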(event EventBeginPlay
  (Variables|Default|SetPlayer%20Character (CallFunction|GetPlayerRef))
  (Game|Player|SetViewTargetwithBlend (Game|GetPlayerController 0) self 0.0 "VTBlend_Linear" 0.0 false))

(event EventTick
  (params (DeltaSeconds :type Float%20%28single-precision%29)))

(fn ConstructionScript)

(fn CamtoPlayerRotation
  (params (InterpSpeed :type Float%20%28single-precision%29))
  (LocalVariables|SetNewLocalVar_0 (Math|Interpolation|RInterpTo (LocalVariables|GetNewLocalVar_0) (Math|Rotator|FindLookatRotation (Transformation|GetWorldLocation (Variables|Default|GetCamera)) (Transformation|GetActorLocation (Variables|Default|GetPlayer%20Character))) (Utilities|Time|GetWorldDeltaSeconds) InterpSpeed))
  (return (LocalVariables|GetNewLocalVar_0)))