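; BP_Spawner is a level utility actor that spawns BP_Collectable actors inside a box volume for the music sports game mode.
; Its SpawnCollectable event picks a random point in the box, spawns a collectable there with itself as Spawner, and increments the game mode's CollectableArray count.
; Nothing in this Blueprint calls that event.
; A count limit check and debug line drawing are present but disconnected, so spawning is uncapped here.
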(event Custom|SpawnCollectable
  (bind _box (Variables|Default|GetBox))
  (bind _game_mode (Variables|Default|GetGame%20Mode))
  (Development|PrintString "Hello0000000" false false "(R=0.000000,G=0.027082,B=1.000000,A=1.000000)" 0.0)
  (Game|SpawnActorfromClass "/Game/_Core/Blueprints/LevelUtility/BP_Collectable.BP_Collectable_C" (Math|Transform|MakeTransform (Math|Random|RandomPointinBoundingBox (Transformation|GetWorldLocation _box) (Components|Box|GetScaledBoxExtent _box)) "0, 0, 0" "1,1,1") "AdjustIfPossibleButAlwaysSpawn" 0 self 0)
  (Variables|/Game/_Core/Blueprints/Manager/GM_MusicSports.GM_MusicSports_C|SetCollectableArray _game_mode (+ (Variables|/Game/_Core/Blueprints/Manager/GM_MusicSports.GM_MusicSports_C|GetCollectableArray _game_mode) 1))
  (Development|PrintString "spawned" false false "(R=0.291187,G=1.000000,B=0.000000,A=1.000000)" 1.0))

(event EventBeginPlay
  (Variables|Default|SetGame%20Mode (CallFunction|GetMusicSportsGameMode)))

(fn ConstructionScript)