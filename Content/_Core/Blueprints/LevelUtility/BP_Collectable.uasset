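; BP_Collectable is a music-sports pickup that is linked to its spawner through a FollowSplineComponent.
; On spawn it caches the player and game mode and attaches a Niagara slash effect.
; A sphere overlap with BP_Char adds score, restores health and decrements the game mode's CollectableArray.
; An overlap with BP_Destroyer counts against the player's health, and either overlap destroys the collectable.
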(event OnComponentBeginOverlap(Sphere1)
  (params (OverlappedComponent :type Primitive%20Component%20Object%20Reference) (OtherActor :type Actor%20Object%20Reference) (OtherComp :type Primitive%20Component%20Object%20Reference) (OtherBodyIndex :type Integer) (bFromSweep :type Boolean) (SweepResult :type Hit%20Result%20Structure%20%28by%20ref%29))
  (bind _game_mode (Variables|Default|GetGame%20Mode))
  (bind _player_character (Variables|Default|GetPlayer%20Character))
  (bind _asbp_char (Utilities|Casting|CastToBP_Char OtherActor)
    (:then
      (Default|ScoreUp _asbp_char)
      (Variables|/Game/_Core/Blueprints/Manager/GM_MusicSports.GM_MusicSports_C|SetCollectableArray _game_mode (- (Variables|/Game/_Core/Blueprints/Manager/GM_MusicSports.GM_MusicSports_C|GetCollectableArray _game_mode) 1))
      (Default|UpdateHealth _player_character 2.0))
    (:CastFailed
      (Utilities|Casting|CastToBP_Destroyer OtherActor)
      (Default|UpdateHealth _player_character -3.0)))
  (Actor|DestroyActor))

(event EventBeginPlay
  (Variables|/Game/_Core/Blueprints/LevelUtility/FollowSplineComponent.FollowSplineComponent_C|SetAs%20BP%20Spawner (Variables|Default|GetFollowSplineComponent) (Variables|Default|GetSpawner))
  (Variables|Default|SetPlayer%20Character (CallFunction|GetPlayerRef))
  (Variables|Default|SetGame%20Mode (CallFunction|GetMusicSportsGameMode))
  (Niagara|SpawnSystemAttached "/Game/AdvancedMagicFX13/Particles/Niagara/NS_ky_hit_slash.NS_ky_hit_slash" (Variables|Default|GetScene) "None" "0, 0, 0" "0, 0, 0" "KeepRelativeOffset" false))

(fn ConstructionScript)