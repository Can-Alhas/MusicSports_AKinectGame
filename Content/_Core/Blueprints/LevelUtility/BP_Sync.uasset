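; BP_Sync is a music-synced light prop that changes its height with beat detection from the music sports game mode's audio analysis.
; Each tick it checks a random band for a beat and interpolates toward a short height on a beat or a tall one otherwise, applying it as the scene root's Z scale.
; The construction script gives the cube a dynamic M_Synclight material tinted by the Color variable.
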(event EventBeginPlay
  (Variables|Default|SetGame%20Mode (CallFunction|GetMusicSportsGameMode)))

(event EventTick
  (params (DeltaSeconds :type Float%20%28single-precision%29))
  (bind _scene (Variables|Default|GetScene))
  (bind _returnvalue (Transformation|GetWorldScale _scene))
  (bind (_x _y) (Math|Vector|BreakVector _returnvalue))
  (Variables|Default|SetCurrent (Math|Interpolation|FInterpTo (Variables|Default|GetCurrent) (Math|Float|SelectFloat 1.0 5.0 (Class|AudioAnalysisToolsLibrary|IsBeat (Variables|/Game/_Core/Blueprints/Manager/GM_MusicSports.GM_MusicSports_C|GetAnalysisRef (Variables|Default|GetGame%20Mode)) (Math|Random|RandomInteger 30))) DeltaSeconds 5.0))
  (Transformation|SetWorldScale3D (Variables|Default|GetScene) (Math|Vector|MakeVector _x _y (Variables|Default|GetCurrent))))

(fn ConstructionScript
  (bind _cube (Variables|Default|GetCube))
  (bind _returnvalue (Rendering|Material|CreateDynamicMaterialInstance _cube 0 "/Game/_Core/Material/SyncLight/M_Synclight.M_Synclight" "None" :!class /Script/Engine.PrimitiveComponent))
  (Variables|Default|SetDynamicMaterial _returnvalue)
  (Rendering|Material|SetMaterial _cube 0 (Variables|Default|GetDynamicMaterial))
  (Rendering|Material|SetVectorParameterValue (Variables|Default|GetDynamicMaterial) "Color" (Variables|Default|GetColor) :!class /Script/Engine.MaterialInstanceDynamic))