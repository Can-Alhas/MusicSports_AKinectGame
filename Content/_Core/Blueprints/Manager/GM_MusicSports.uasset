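; Music Sports manager Blueprint that plays a music track and signals its beats to the game at runtime.
; On BeginPlay it imports an MP3 from a hardcoded local path through Runtime Audio Importer and creates a Hanning-windowed audio analyzer.
; Generated PCM data from the playing sound feeds beat detection, calling BeatUpdate whenever the checked band registers a beat.
; Unconnected debug-print and older amplitude-sampling nodes remain.
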(event Custom|Result
  (params (RuntimeAudioImporterObjectRef :type Runtime%20Audio%20Importer%20Library%20Object%20Reference) (SoundWaveRef :type Imported%20Sound%20Wave%20Object%20Reference) (Status :type ETranscodingStatus%20Enum :default "SuccessfulImport"))
  (if (Utilities|Enum|Equal(Enum) Status "SuccessfulImport")
    (EventDispatchers|BindEventtoOnGeneratePCMData SoundWaveRef (delegate Custom|PCMDataGen))
    (Audio|PlaySound2D SoundWaveRef 1.0 1.0 0.0 0 0)))

(event Custom|PCMDataGen
  (params (PCMData :type Array%20of%20Floats%20%28single-precision%29))
  (Class|AudioAnalysisToolsLibrary|ProcessAudioFrame (Variables|Default|GetAnalysisRef) PCMData true)
  (if (Class|AudioAnalysisToolsLibrary|IsBeat (Variables|Default|GetAnalysisRef) 20)
    (Default|CallBeatUpdate)))

(event EventBeginPlay
  (Utilities|FlowControl|Sequence
    (:then_0
      (bind _returnvalue (Class|RuntimeAudioImporterLibrary|CreateRuntimeAudioImporter))
      (Variables|Default|SetImporterRef _returnvalue)
      (EventDispatchers|BindEventtoOnResult (Variables|Default|GetImporterRef) (delegate Custom|Result))
      (Class|RuntimeAudioImporterLibrary|ImportAudiofromFile (Variables|Default|GetImporterRef) "C:\\MyWorkspace\\SocialWorksDepot\\MusicSports\\ExternalData\\fade.mp3" "Mp3")
      (bind _returnvalue_2 (Class|AudioAnalysisToolsLibrary|CreateAudioAnalysisTools 4096 "HanningWindow"))
      (Variables|Default|SetAnalysisRef _returnvalue_2))))

(fn ConstructionScript)