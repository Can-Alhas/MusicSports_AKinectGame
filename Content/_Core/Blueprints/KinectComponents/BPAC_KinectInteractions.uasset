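; Actor component that turns the nearest tracked Kinect body into gesture events and hand-axis input.
; Each tick it checks hand distance and state, firing edge-triggered events for both hands open or closed.
; Single and double claps share a counter reset by a retriggerable delay, so single fires before double.
; Interpolated wrist forward-vector Z values are broadcast per hand and summed; sensor init and uninit are unwired.
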(event Custom|HandClapCheck
  ;[1 1 1] Comment
  ;;[1 1 1] SingleClap
  (if (<= (Class|NeoKinectBody|GetJointsDistance (Variables|Default|GetNearestBody) "HandLeft" "HandRight") (Variables|Default|GetDistance%20Threshold))
    (Utilities|FlowControl|DoOnce false :!label _label)
    (else
      (goto _label Reset))))

(event Custom|DoubleHandClapCheck
  (bind _distance_threshold (Variables|Default|GetDistance%20Threshold))
  (bind _nearestbody (Variables|Default|GetNearestBody))
  (bind _returnvalue (Class|NeoKinectBody|GetJointsDistance _nearestbody "HandLeft" "HandRight"))
  (bind _returnvalue_2 (<= _returnvalue _distance_threshold))
  ;[1 1 1] Comment
  ;;[1 1 1] DoubleClap
  (if _returnvalue_2
    (Utilities|FlowControl|DoOnce _returnvalue_2 :!label _label
      (:Completed
        (Utilities|FlowControl|Sequence
          (:then_0
            (bind _result (Math|Integer|IncrementInt (Variables|Default|GetDoubleClapCounter))
              (:%20%20
                (Variables|Default|SetDoubleClapCounter _result)
                (bind _counter (Utilities|FlowControl|DoN (Variables|Default|GetDoubleClapCounter) :!label _label_2)
                  (:Exit
                    (switch int _counter
                      (:1
                        (Default|CallEventonSingleHandClap))
                      (:2
                        (Default|CallEventonDoubleHandClap))))))))
          (:then_1
            (Utilities|FlowControl|RetriggerableDelay (Variables|Default|GetHandClampResetTimer))
            (Variables|Default|SetDoubleClapCounter (Variables|Default|GetDoubleClapCounter))
            (goto _label_2 Reset)))))
    (else
      (goto _label Reset))))

(event Custom|HandOpenCheck
  ;[1 1 1] Comment
  ;;[1 1 1] HandOpened
  (if (CallFunction|TwoHandStateCheck (Variables|Default|GetNearestBody) "Open")
    (Utilities|FlowControl|DoOnce true :!label _label
      (:Completed
        (Default|CallEventonHandsOpened)))
    (else
      (goto _label Reset))))

(event Custom|HandCloseCheck
  ;[1 1 1] Comment
  ;;[1 1 1] HandClosed
  (if (CallFunction|TwoHandStateCheck (Variables|Default|GetNearestBody) "Closed")
    (Utilities|FlowControl|DoOnce true :!label _label
      (:Completed
        (Default|CallEventonHandsClosed)))
    (else
      (goto _label Reset))))

(event Custom|UpdateHandController
  (params (InterpSpeed :type Float%20%28single-precision%29))
  ;[1 1 1] Comment
  ;;[1 1 1] AxisController
  (bind _returnvalue (CallFunction|GetJointForwardAxis "WristRight" InterpSpeed))
  (bind _returnvalue_2 (CallFunction|GetJointForwardAxis "WristLeft" InterpSpeed))
  (bind _output_get (Variables|Default|SetHandControllerReturn (+ _returnvalue_2 _returnvalue)))
  (Default|CallHandControllerAxisInput _output_get)
  (Default|CallHandAxis _returnvalue_2 _returnvalue))

(event EventTick
  (params (DeltaSeconds :type Float%20%28single-precision%29))
  (bind _returnvalue (Class|NeoKinectManager|GetNearestBody))
  ;[1 1 1] Comment
  ;;[1 1 1] MainControl
  (if (Class|NeoKinectManager|IsKinectAvailable)
    (Utilities|IsValid _returnvalue
      (:Is%20Valid
        (if (Variables|/Script/NeoKinectUnreal.NeoKinectBody|GetbIsTracked _returnvalue)
          (Variables|Default|SetNearestBody _returnvalue)
          (Utilities|FlowControl|Sequence
            (:then_0
              (CallFunction|HandClapCheck)
              (CallFunction|DoubleHandClapCheck))
            (:then_1
              (CallFunction|HandOpenCheck)
              (CallFunction|HandCloseCheck))
            (:then_2
              (CallFunction|UpdateHandController (Variables|Default|GetInterp%20Speed)))))))))

(event EventBeginPlay
  ;[1 1 1] Comment
  ;;[1 1 1] Init & Uninit
)

(event EventEndPlay
  (params (EndPlayReason :type EEndPlayReason%20Enum :default "Destroyed"))
  ;[1 1 1] Comment
  ;;[1 1 1] Init & Uninit
)

(fn TwoHandStateCheck
  (params (KinectBodyObject :type Neo%20Kinect%20Body%20Object%20Reference) (State :type EKinectHandState%20Enum :default "Unknown"))
  (return (and (Utilities|Enum|Equal(Enum) (Class|NeoKinectBody|GetHandState KinectBodyObject "Left") State) (Utilities|Enum|Equal(Enum) (Class|NeoKinectBody|GetHandState KinectBodyObject "Right") State))))

(fn GetJointForwardAxis
  (params (Joint :type EKinectJointType%20Enum :default "SpineBase") (InterpSpeed :type Float%20%28single-precision%29))
  (bind _output_get (LocalVariables|SetCurrent (Math|Interpolation|FInterpTo (LocalVariables|GetCurrent) (.z (Math|Vector|GetForwardVector (Class|NeoKinectBody|GetJointOrientation (Variables|Default|GetNearestBody) Joint))) (Utilities|Time|GetWorldDeltaSeconds) InterpSpeed)))
  (return _output_get))

(fn PitchCalc
  (params (Current :type Float%20%28single-precision%29))
  (return (Math|Interpolation|FInterpTo Current (/ (+ (Variables|Default|GetLeftZ) (* (Variables|Default|GetRightZ%20) -1.0)) 2.0) (Utilities|Time|GetWorldDeltaSeconds) (Variables|Default|GetInterp%20Speed))))