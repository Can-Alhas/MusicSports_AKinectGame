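; Player character driven by Kinect body tracking, with health, a score counter and game over.
; Tick eases the avateering AnimBP's joint transforms toward the nearest body's joints with a delta-time lerp, searching again when that body is invalid.
; Hand controller axis input sweeps the actor along world X.
; Zero health hides the mesh and board, pauses the game and shows the game-over widget.
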(event HandControllerAxisInput(BPAC_KinectInteractions)
  (params (AxisReturn :type Float%20%28single-precision%29))
  (Transformation|AddActorWorldOffset (Math|Vector|MakeVector (* AxisReturn -5e+01) 0.0 0.0) true))

(event EventBeginPlay
  (Utilities|FlowControl|Sequence
    (:then_0
      (bind _asavateering_demo_anim_bp (Utilities|Casting|CastToAvateeringDemo_AnimBP (Components|SkeletalMesh|GetAnimInstance (Variables|Character|GetMesh))))
      (Variables|Default|SetAvateeringAnims _asavateering_demo_anim_bp)
      (Variables|Default|SetkinectBody (.ReturnValue (Class|NeoKinectManager|GetNearestBody))))
    (:then_1
      (bind _returnvalue (UserInterface|CreateWidget "/Game/_Core/UMG/Widget_PlayerHealth.Widget_PlayerHealth_C"))
      (UserInterface|Viewport|AddtoViewport _returnvalue 0))))

(event EventTick
  (params (DeltaSeconds :type Float%20%28single-precision%29))
  (bind _avateeringanims (Variables|Default|GetAvateeringAnims))
  (bind _jointstransform (Variables|/Game/NeoKinectDemos/Blueprints/AvateeringDemo_AnimBP.AvateeringDemo_AnimBP_C|GetJointsTransform _avateeringanims))
  (if (Class|NeoKinectManager|IsKinectAvailable)
    (Variables|Default|GetkinectBody
      (:then
        (for (_array_element _array_index) (Class|NeoKinectBody|GetJoints (Variables|Default|GetkinectBody))
          (Utilities|Array|SetArrayElem _jointstransform _array_index (Math|Transform|Lerp(Transform) (Utilities|Array|Get(acopy) _jointstransform _array_index) (Math|Transform|MakeTransform (.Location (Utilities|Struct|BreakKinectJoint _array_element)) (.Orientation (Utilities|Struct|BreakKinectJoint _array_element))) (Math|Float|Min(Float) (* (Utilities|Time|GetWorldDeltaSeconds) 1e+01) 1.0)))))
      (:else
        (Variables|Default|SetkinectBody (.ReturnValue (Class|NeoKinectManager|GetNearestBody)))))))

(fn ConstructionScript)

(fn UpdateHealth
  (params (HealthChanges :type Float%20%28single-precision%29))
  (Variables|Default|SetHealth (Math|Float|Clamp(Float) (+ (Variables|Default|GetHealth) HealthChanges) 0.0 (Variables|Default|GetMaxHealth)))
  (Utilities|FlowControl|Sequence
    (:then_0
      (if (== (Variables|Default|GetHealth) 0.0)
        (CallFunction|Dead)))
    (:then_1
      (if (> HealthChanges 0.0)
        _))))

(fn Dead
  (Rendering|SetVisibility (Variables|Character|GetMesh) false false)
  (Variables|Default|SetIsAlive true)
  (Game|SetGamePaused true)
  (bind _returnvalue (UserInterface|CreateWidget "/Game/_Core/UMG/Widget_GameOver.Widget_GameOver_C"))
  (UserInterface|Viewport|AddtoViewport _returnvalue 0))

(fn ScoreUp
  (Variables|Default|SetScore (+ (Variables|Default|GetScore) 1)))